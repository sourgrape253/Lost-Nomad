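; MovingPlatform_ChildUP is a child moving-platform Blueprint that shifts its Platform component along world Y, despite the UP in its name.
; Every Tick calls the parent Tick, then restarts the ForwardandBack timeline from the start.
; Timeline updates add the LeftandRightMovement track, scaled by LRMovementAmount, to the current Y without sweeping, so movement is cumulative.
; Similar X and Z offset calculations are left unused.
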(event `self.ReceiveTick`
  (params (DeltaSeconds :type "Float (single-precision)"))
  (`parent.ReceiveTick` DeltaSeconds)
  (bind (_direction _leftandrightmovement) (`Timeline|ForwardandBack` :`NewTime` 10.0 :!via `PlayFromStart`)
    (:`Update`
      (`SceneComponent.K2_SetWorldLocation` (`self.Platform`) (`KismetMathLibrary.MakeVector` (.x (`SceneComponent.K2_GetComponentLocation` (`self.Platform`))) (+ (* _leftandrightmovement (`self.L&RMovementAmount`)) (.y (`SceneComponent.K2_GetComponentLocation` (`self.Platform`)))) (.z (`SceneComponent.K2_GetComponentLocation` (`self.Platform`)))) false false))))

(fn `UserConstructionScript`
  (`parent.UserConstructionScript`))