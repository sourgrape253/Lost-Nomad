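; Master Blueprint for moving platforms that selects timeline-driven motion values from actor tags.
; Each tick, UpDownHold, DownUp and LEftRight tags play separate timelines, the first two writing their curve outputs into TimelineArray and Upanddown.
; It appears unfinished: the LEftRight timeline has no update logic, some branches are empty or unreachable, and nothing in these graphs moves the actor.
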(event `self.ReceiveBeginPlay`)

(event `self.ReceiveTick`
  (params (DeltaSeconds :type "Float (single-precision)"))
  (`|ExecutionSequence`
    (:`then_0`
      (if (`self.ActorHasTag` "UpDownHold")
        (bind (_direction _updownhold _downuphold _updowneven) (`Timeline|test`)
          (:`Update`
            (set `self.TimelineArray` (`|MakeArray` _updownhold _downuphold _updowneven 0.0))))))
    (:`then_1`
      (if (`self.ActorHasTag` "DownUp")
        (bind (_direction_2 _updownhold_2) (`Timeline|Timeline_1`)
          (:`Update`
            (set `self.upanddown` _updownhold_2)))))
    (:`then_2`
      (if (`self.ActorHasTag` "LEftRight")
        (`Timeline|Timeline_2`)))
    (:`then_3`
      (if true
        _))
    (:`then_4`
      (if true
        _))))

(fn `UserConstructionScript`)