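; MovingPlatformParent is a platform Blueprint, named as a parent class, that moves its Platform component through the world with a timeline.
; Tick calls Play on the MoveBackandForward timeline, whose MoveLeftRight track is scaled by MovementAmount.
; Each update adds that same offset to the current world X, Y and Z without sweeping, so movement accumulates rather than following a fixed origin.
; The construction script is empty, and MoveCode is an unused stub returning zeros.
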(event `self.ReceiveTick`
  (params (DeltaSeconds :type "Float (single-precision)"))
  (bind (_direction _move_left_right) (`Timeline|MoveBackandForward` :`NewTime` 20.0)
    (:`Update`
      (bind _returnvalue (* _move_left_right (`self.Movement Amount`)))
      (`SceneComponent.K2_SetWorldLocation` (`self.Platform`) (`KismetMathLibrary.MakeVector` (+ _returnvalue (.x (`SceneComponent.K2_GetComponentLocation` (`self.Platform`)))) (+ _returnvalue (.y (`SceneComponent.K2_GetComponentLocation` (`self.Platform`)))) (+ _returnvalue (.z (`SceneComponent.K2_GetComponentLocation` (`self.Platform`))))) false false))))

(fn `MoveCode`
  (params (TimelineValue :type "Float (double-precision)"))
  (returns (Vector :type "Vector Structure"))
  (return (0.0 0.0 0.0)))

(fn `UserConstructionScript`)